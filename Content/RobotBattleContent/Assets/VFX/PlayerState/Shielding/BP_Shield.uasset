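; Shield VFX Blueprint that drives a Niagara shield from the robot's guard events.
; Raising the guard reinitializes the system; lowering it jumps particle age, then deactivates after a short delay.
; Each hit spikes a color modifier and starts fading the next of four particle groups, with no reset after BeginPlay.
; Tick decays these values and streams them to Niagara through the NDC_Shield data channel.
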(event Custom|CE_OnShieldBroughtUp
  (Niagara|ReinitializeSystem (Variables|Default|GetNiagara)))

(event Custom|CE_OnShieldDown
  (Niagara|SetNiagaraVariable(Float) (Variables|Default|GetNiagara) "Particles.Age" 149.7)
  (Utilities|FlowControl|Delay 0.4)
  (Components|Activation|Deactivate (Variables|Default|GetNiagara)))

(event Custom|CE_OnShieldHit
  (Variables|Default|SetShieldHitColorModifier 1e+01)
  (bind _index (CallFunction|GetCurrentGroupIndex))
  (CallFunction|WritefromCurrentGroupIndex _index)
  (|WriteDataChannel :Channel "/Game/RobotBattleContent/Assets/VFX/PlayerState/Shielding/NDC_Shield.NDC_Shield" :GroupActivationMults (Variables|Default|GetGroupActivationMults) :ShieldHitColorModifier (Variables|Default|GetShieldHitColorModifier)))

(event Custom|CE_Guard
  (params (GuardLeft :type Integer))
  (CallFunction|CEonShieldHit))

(event Custom|CE_GuardManager
  (params (Guard :type Boolean))
  (if Guard
    (CallFunction|CEonShieldBroughtUp)
    (else
      (CallFunction|CEonShieldDown))))

(event EventBeginPlay
  (bind _robot (Variables|Default|GetRobot))
  (bind _output_get (Variables|Default|SetGroupActivationMults (Math|Vector4|MakeVector4 1.0 1.0 1.0 1.0)))
  (|WriteDataChannel :Channel "/Game/RobotBattleContent/Assets/VFX/PlayerState/Shielding/NDC_Shield.NDC_Shield" :GroupActivationMults _output_get)
  (EventDispatchers|AssignGuardEvent _robot (delegate Custom|CE_Guard))
  (EventDispatchers|AssignGuardManagerEvent _robot (delegate Custom|CE_GuardManager)))

(event EventTick
  (params (DeltaSeconds :type Float%20%28single-precision%29))
  (bind _output_get (Variables|Default|SetShieldHitColorModifier (- (Variables|Default|GetShieldHitColorModifier) DeltaSeconds)))
  (if (< _output_get 0.0)
    (Variables|Default|SetShieldHitColorModifier 0.0))
  (CallFunction|DecreaseMultsasNeeded DeltaSeconds)
  (|WriteDataChannel :Channel "/Game/RobotBattleContent/Assets/VFX/PlayerState/Shielding/NDC_Shield.NDC_Shield" :GroupActivationMults (Variables|Default|GetGroupActivationMults) :ShieldHitColorModifier (Variables|Default|GetShieldHitColorModifier)))

(fn ConstructionScript)

(fn GetCurrentGroupIndex
  (bind _groupactivationmults (Variables|Default|GetGroupActivationMults))
  (if (>= (.x _groupactivationmults) 1.0)
    (return 1)
    (elif (>= (.y _groupactivationmults) 1.0)
      (return 2)
      (elif (>= (.z _groupactivationmults) 1.0)
        (return 3)
        (elif (>= (.w _groupactivationmults) 1.0)
          (return 4))))))

(fn WritefromCurrentGroupIndex
  (params (Index :type Integer))
  (switch int Index
    (:1
      (Variables|Default|SetGroupActivationMults (Math|Vector4|MakeVector4 0.99 (.y (Variables|Default|GetGroupActivationMults)) (.z (Variables|Default|GetGroupActivationMults)) (.w (Variables|Default|GetGroupActivationMults)))))
    (:2
      (Variables|Default|SetGroupActivationMults (Math|Vector4|MakeVector4 (.x (Variables|Default|GetGroupActivationMults)) 0.99 (.z (Variables|Default|GetGroupActivationMults)) (.w (Variables|Default|GetGroupActivationMults)))))
    (:3
      (Variables|Default|SetGroupActivationMults (Math|Vector4|MakeVector4 (.x (Variables|Default|GetGroupActivationMults)) (.y (Variables|Default|GetGroupActivationMults)) 0.99 (.w (Variables|Default|GetGroupActivationMults)))))
    (:4
      (Variables|Default|SetGroupActivationMults (Math|Vector4|MakeVector4 (.x (Variables|Default|GetGroupActivationMults)) (.y (Variables|Default|GetGroupActivationMults)) (.z (Variables|Default|GetGroupActivationMults)) 0.99)))))

(fn DecreaseMultsasNeeded
  (params (DeltaSeconds :type Float%20%28double-precision%29))
  (if (< (.x (Variables|Default|GetGroupActivationMults)) 1.0)
    (Variables|Default|SetGroupActivationMults (Math|Vector4|MakeVector4 (- (.x (Variables|Default|GetGroupActivationMults)) DeltaSeconds) (.y (Variables|Default|GetGroupActivationMults)) (.z (Variables|Default|GetGroupActivationMults)) (.w (Variables|Default|GetGroupActivationMults)))))
  (if (< (.y (Variables|Default|GetGroupActivationMults)) 1.0)
    (Variables|Default|SetGroupActivationMults (Math|Vector4|MakeVector4 (.x (Variables|Default|GetGroupActivationMults)) (- (.y (Variables|Default|GetGroupActivationMults)) DeltaSeconds) (.z (Variables|Default|GetGroupActivationMults)) (.w (Variables|Default|GetGroupActivationMults)))))
  (if (< (.z (Variables|Default|GetGroupActivationMults)) 1.0)
    (Variables|Default|SetGroupActivationMults (Math|Vector4|MakeVector4 (.x (Variables|Default|GetGroupActivationMults)) (.y (Variables|Default|GetGroupActivationMults)) (- (.z (Variables|Default|GetGroupActivationMults)) DeltaSeconds) (.w (Variables|Default|GetGroupActivationMults)))))
  (if (< (.w (Variables|Default|GetGroupActivationMults)) 1.0)
    (Variables|Default|SetGroupActivationMults (Math|Vector4|MakeVector4 (.x (Variables|Default|GetGroupActivationMults)) (.y (Variables|Default|GetGroupActivationMults)) (.z (Variables|Default|GetGroupActivationMults)) (- (.w (Variables|Default|GetGroupActivationMults)) DeltaSeconds)))))