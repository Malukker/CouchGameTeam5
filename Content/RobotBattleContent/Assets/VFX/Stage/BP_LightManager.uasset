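; Stage light manager that moves two spotlights to follow the first two RobotCharacterDown actors found at BeginPlay.
; Each tick, it inverse-lerps world X zero between the characters' average X and the viewport's minimum-bound X.
; Below TwoLightsThreshold, each spotlight takes its character's X and Z, keeping its own Y.
; The one-light transition is unfinished: its branches are empty, vertical offset and lerp are unused, and FollowPlayers and ScaleWithDistance are stubs.
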(event EventBeginPlay
  (bind _outactors (Actor|GetAllActorsOfClass "/Script/RobotBattle.RobotCharacterDown"))
  (Variables|Default|SetCharacters _outactors))

(event EventTick
  (params (DeltaSeconds :type Float%20%28single-precision%29))
  (bind _returnvalue (Subsystems|GetCameraWorldSubsystem))
  (bind _characters (Variables|Default|GetCharacters))
  (bind _characters_2 (Variables|Default|GetCharacters))
  (bind _output (Utilities|Array|Get(acopy) _characters 1))
  (bind _output_2 (Utilities|Array|Get(acopy) _characters_2))
  (bind _returnvalue_2 (Transformation|GetActorLocation _output))
  (bind _returnvalue_3 (Transformation|GetActorLocation _output_2))
  (bind _barycentre (CallFunction|CalculateAveragePositionBetweenTargets))
  (Variables|Default|SetBoundsCenterX (.X (Math|Vector|BreakVector _barycentre)))
  (bind _outviewportboundsmin (Class|CameraWorldSubsystem|GetViewportBounds _returnvalue))
  (bind _returnvalue_4 (Class|CameraWorldSubsystem|CalculateWorldPositionfromViewportPosition _returnvalue _outviewportboundsmin))
  (Variables|Default|SetBoundsExtentX (.X (Math|Vector|BreakVector _returnvalue_4)))
  (if (< (/ (- 0.0 (Variables|Default|GetBoundsCenterX)) (- (Variables|Default|GetBoundsExtentX) (Variables|Default|GetBoundsCenterX))) (Variables|Default|GetTwoLightsThreshold))
    (Transformation|SetWorldLocation (Variables|Default|GetSpotLight1) (Math|Vector|MakeVector (.x _returnvalue_3) (.y (Transformation|GetWorldLocation (Variables|Default|GetSpotLight1))) (.z _returnvalue_3)) false false)
    (Transformation|SetWorldLocation (Variables|Default|GetSpotLight2) (Math|Vector|MakeVector (.x _returnvalue_2) (.y (Transformation|GetWorldLocation (Variables|Default|GetSpotLight2))) (.z _returnvalue_2)) false false)
    (elif (and (>= (/ (- 0.0 (Variables|Default|GetBoundsCenterX)) (- (Variables|Default|GetBoundsExtentX) (Variables|Default|GetBoundsCenterX))) (Variables|Default|GetTwoLightsThreshold)) (<= (/ (- 0.0 (Variables|Default|GetBoundsCenterX)) (- (Variables|Default|GetBoundsExtentX) (Variables|Default|GetBoundsCenterX))) (Variables|Default|GetOneLightThreshold)))
      _)))

(fn ConstructionScript)

(fn CalculateAveragePositionBetweenTargets
  (for _array_element (Variables|Default|GetCharacters)
    (bind _output_get (LocalVariables|SetTargetPos (Transformation|GetActorLocation _array_element)))
    (LocalVariables|SetNewPos (+ _output_get (LocalVariables|GetNewPos)))
    (LocalVariables|SetTargetsAmount (+ 1 (LocalVariables|GetTargetsAmount))))
  (bind _output_get_2 (LocalVariables|SetNewPos (/ (LocalVariables|GetNewPos) (LocalVariables|GetTargetsAmount))))
  (return _output_get_2))

(fn FollowPlayers)

(fn ScalewithDistance)