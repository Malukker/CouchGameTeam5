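; BP_RobotBounds places two side boxes, BoxLeft and BoxRight, from the bounds of a referenced Bounds actor.
; The Construction Script feeds that actor's vertical extent into both boxes' size and world height.
; Both boxes take the bounds' Y origin, while their X positions derive from the X extent alone, ignoring the X origin.
; It has no runtime logic, as all event nodes are disabled stubs.
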(event EventBeginPlay)

(event Collision|EventActorBeginOverlap
  (params (OtherActor :type Actor%20Object%20Reference)))

(event EventTick
  (params (DeltaSeconds :type Float%20%28single-precision%29)))

(fn ConstructionScript
  (bind _bounds (Variables|Default|GetBounds))
  (bind (_origin _boxextent) (Collision|GetActorBounds _bounds false false))
  (bind (_x _y _z) (Math|Vector|BreakVector _boxextent))
  (bind _y_2 (Math|Vector|BreakVector _origin))
  (bind _z_2 (Math|Vector|BreakVector _boxextent))
  (Components|Box|SetBoxExtent (Variables|Default|GetBox_Left) (Math|Vector|MakeVector 0.0 0.0 _z_2) false)
  (Components|Box|SetBoxExtent (Variables|Default|GetBox_Right) (Math|Vector|MakeVector 0.0 0.0 _z_2) false)
  (bind _result (Math|Float|NegateFloat _x)
    (:%20%20
      (Transformation|SetWorldLocation (Variables|Default|GetBox_Left) (Math|Vector|MakeVector _result _y_2 _z) false false)
      (Transformation|SetWorldLocation (Variables|Default|GetBox_Right) (Math|Vector|MakeVector _x _y_2 _z) false false))))