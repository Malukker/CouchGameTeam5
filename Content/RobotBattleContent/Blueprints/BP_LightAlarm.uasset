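; BP_LightAlarm is an alarm light that flashes red when round 2 starts.
; It binds to the MatchManager's round start event and plays a timeline that drives the light's green and blue channels, tinting it between white and red.
; A delayed end event resets the light to white and stops the timeline after a few seconds.
; A separate Test event also plays the timeline.
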(event Custom|Test
  (bind _color (Timeline|Timeline Play)
    (:Update
      (Rendering|Components|Light|SetLightColor (Variables|/Script/Engine.Light|GetLightComponent (Variables|Default|GetLight)) (Utilities|Struct|MakeLinearColor 1.0 _color _color 1.0) true))))

(event Custom|CE_End
  (Utilities|FlowControl|Delay 4.0)
  (Rendering|Components|Light|SetLightColor (Variables|/Script/Engine.Light|GetLightComponent (Variables|Default|GetLight)) "(R=1.000000,G=1.000000,B=1.000000,A=1.000000)" true)
  (bind _color (Timeline|Timeline Stop)
    (:Update
      (Rendering|Components|Light|SetLightColor (Variables|/Script/Engine.Light|GetLightComponent (Variables|Default|GetLight)) (Utilities|Struct|MakeLinearColor 1.0 _color _color 1.0) true))))

(event Custom|CE_Alarm
  (params (Round :type Integer))
  (if (== Round 2)
    (CallFunction|CEEnd)
    (bind _color (Timeline|Timeline Play)
      (:Update
        (Rendering|Components|Light|SetLightColor (Variables|/Script/Engine.Light|GetLightComponent (Variables|Default|GetLight)) (Utilities|Struct|MakeLinearColor 1.0 _color _color 1.0) true)))))

(event EventBeginPlay
  (bind _returnvalue (Actor|GetActorOfClass "/Script/RobotBattle.MatchManager"))
  (EventDispatchers|BindEventtoRoundStartEvent _returnvalue (delegate Custom|CE_Alarm)))

(fn ConstructionScript)