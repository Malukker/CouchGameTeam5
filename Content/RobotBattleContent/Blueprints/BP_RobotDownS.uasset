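; BP_RobotDownS is a robot Blueprint that equips itself with a shield and sets its team material when play begins.
; On BeginPlay it spawns a BP_Shield, snaps it to the ShieldPos component and passes itself as the shield's Robot reference.
; After a one-tick delay, it picks the first material slot of its mesh from two options based on Team.
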(event EventBeginPlay
  (bind _returnvalue (Game|SpawnActorfromClass "/Game/RobotBattleContent/Assets/VFX/PlayerState/Shielding/BP_Shield.BP_Shield_C" (Math|Transform|MakeTransform "0, 0, 0" "0, 0, 0" "1.000000,1.000000,1.000000") "AlwaysSpawn" "MultiplyWithRoot" 0 0))
  (Transformation|AttachComponentToComponent (Variables|/Script/Engine.Actor|GetRootComponent _returnvalue) (Variables|Default|GetShieldPos) "None" "SnapToTarget" "SnapToTarget" "SnapToTarget" false)
  (Variables|/Game/RobotBattleContent/Assets/VFX/PlayerState/Shielding/BP_Shield.BP_Shield_C|SetRobot _returnvalue self)
  (Utilities|FlowControl|DelayUntilNextTick)
  (Rendering|Material|SetMaterial (Variables|Character|GetMesh) 0 (Utilities|Select :Index (Variables|Default|GetTeam) :Option%200 "/Game/RobotBattleContent/Assets/Textures/RobotTexture/Bas_S/Team1/M_DownS_T1.M_DownS_T1" :Option%201 "/Game/RobotBattleContent/Assets/Textures/RobotTexture/Bas_S/Default/M_Bas_S.M_Bas_S")))

(fn ConstructionScript)