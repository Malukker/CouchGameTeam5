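; BP_RobotUpL is a robot Blueprint, apparently the upper-left variant, that carries a shield and shows team-specific visuals.
; On BeginPlay it spawns a BP_Shield, snaps it to ShieldPos and gives it a back-reference to the robot.
; One tick later it sets the mesh material by Team and, when IsLookingOpponent is true, also sets the matching team sprite.
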(event EventBeginPlay
  (bind _returnvalue (Game|SpawnActorfromClass "/Game/RobotBattleContent/Assets/VFX/PlayerState/Shielding/BP_Shield.BP_Shield_C" (Math|Transform|MakeTransform "0, 0, 0" "0, 0, 0" "1.000000,1.000000,1.000000") "AlwaysSpawn" "MultiplyWithRoot" 0 0))
  (Transformation|AttachComponentToComponent (Variables|/Script/Engine.Actor|GetRootComponent _returnvalue) (Variables|Default|GetShieldPos) "None" "SnapToTarget" "SnapToTarget" "SnapToTarget" false)
  (Variables|/Game/RobotBattleContent/Assets/VFX/PlayerState/Shielding/BP_Shield.BP_Shield_C|SetRobot _returnvalue self)
  (Utilities|FlowControl|DelayUntilNextTick)
  (Rendering|Material|SetMaterial (Variables|Character|GetMesh) 0 (Utilities|Select :Index (Variables|Default|GetTeam) :Option%200 "/Game/RobotBattleContent/Assets/Textures/RobotTexture/Top_L/Team1/M_Top_L_T1.M_Top_L_T1" :Option%201 "/Game/RobotBattleContent/Assets/Textures/RobotTexture/Top_L/Team2/M_TopL_T2.M_TopL_T2"))
  (if (Variables|Default|GetIsLookingOpponent)
    (Rendering|Components|Sprite|SetSprite (Variables|Default|GetTeamSprite) (Utilities|Select :Index (Variables|Default|GetTeam) :Option%200 "/Game/RobotBattleContent/Assets/Team/T_1_Sprite.T_1_Sprite" :Option%201 "/Game/RobotBattleContent/Assets/Team/T_2_Sprite1.T_2_Sprite1"))))

(fn ConstructionScript)