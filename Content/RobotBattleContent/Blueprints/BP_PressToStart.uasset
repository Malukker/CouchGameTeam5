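; Press-to-start actor that runs the menu's opening transition into team selection.
; It listens for input from all BP_PlayerMenuActors; the first press swaps the current level sequence for Ouverture_Anim.
; After a fixed delay, it opens WBP_TeamSelectionMenu, narrows the camera FOV, unbinds input and destroys intro actors.
; When the GameInstance's ChangeCharacter flag is set, it skips straight to cleanup and FOV, clearing the flag without creating the menu.
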(event Custom|CE_KeyPressed
  (if (not (Variables|Default|GetClicked))
    (Variables|Default|SetClicked true)
    (Sequencer|Player|Stop (Variables|/Script/LevelSequence.LevelSequenceActor|GetSequencePlayer (Variables|Default|GetAnimCurrent)) :!class /Script/MovieScene.MovieSceneSequencePlayer)
    (bind (_outactor _returnvalue) (Sequencer|Player|CreateLevelSequencePlayer "/Game/RobotBattleContent/Animation/Main_Menu/Ouverture_Anim.Ouverture_Anim"))
    (Variables|Default|SetAnimCurrent _outactor)
    (Sequencer|Player|Play _returnvalue :!class /Script/MovieScene.MovieSceneSequencePlayer)
    (Utilities|FlowControl|Delay 3.0)
    (CallFunction|CEFinishAnim)))

(event Custom|CE_DestroyAll
  (for _array_element (Variables|Default|GetOut%20Actors)
    (EventDispatchers|UnbindallEventsfromOnInput _array_element))
  (for _array_element_2 (Variables|Default|GetDestroyOnEnd)
    (Actor|DestroyActor _array_element_2)))

(event Custom|CE_FinishAnim
  (Actor|DestroyActor (Variables|Default|GetAnimCurrent))
  (bind _returnvalue (UserInterface|CreateWidget "/Game/RobotBattleContent/UI/WBP_TeamSelectionMenu.WBP_TeamSelectionMenu_C"))
  (UserInterface|Viewport|AddtoViewport _returnvalue 0)
  (Camera|SetFieldOfView (Variables|/Script/Engine.CameraActor|GetCameraComponent (Variables|Default|GetCamera)) 17.0)
  (for _array_element (Variables|Default|GetOut%20Actors)
    (EventDispatchers|UnbindallEventsfromOnInput _array_element))
  (for _array_element_2 (Variables|Default|GetDestroyOnEnd)
    (Actor|DestroyActor _array_element_2)))

(event EventBeginPlay
  (Utilities|FlowControl|Delay 0.5)
  (bind _outactors (Actor|GetAllActorsOfClass "/Game/RobotBattleContent/Blueprints/BP_PlayerMenuActor.BP_PlayerMenuActor_C"))
  (Variables|Default|SetOut%20Actors _outactors)
  (bind _asgi_robot_battle (Utilities|Casting|CastToGI_RobotBattle (Game|GetGameInstance)))
  (bind _returnvalue (Class|RobotGameInstance|GetChangeCharacter _asgi_robot_battle))
  (if _returnvalue
    (CallFunction|CEDestroyAll)
    (Camera|SetFieldOfView (Variables|/Script/Engine.CameraActor|GetCameraComponent (Variables|Default|GetCamera)) 17.0)
    (Class|RobotGameInstance|SetChangeCharacter _asgi_robot_battle false)
    (else
      (for _array_element (Variables|Default|GetOut%20Actors)
        (EventDispatchers|BindEventtoOnInput _array_element (delegate Custom|CE_KeyPressed))))))

(fn ConstructionScript)