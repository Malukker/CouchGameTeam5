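; BP_RobotUpS is a robot upper part in RobotBattle that carries a shield and shows its team's look.
; On BeginPlay it spawns a BP_Shield, snaps it to the ShieldPos component and passes itself as the shield's Robot reference.
; It then uses the Team value to choose the team sprite and the mesh material.
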(event EventBeginPlay
  (bind _returnvalue (Game|SpawnActorfromClass "/Game/RobotBattleContent/Assets/VFX/PlayerState/Shielding/BP_Shield.BP_Shield_C" (Math|Transform|MakeTransform "0, 0, 0" "0, 0, 0" "1.000000,1.000000,1.000000") "AlwaysSpawn" "MultiplyWithRoot" 0 0))
  (Transformation|AttachComponentToComponent (Variables|/Script/Engine.Actor|GetRootComponent _returnvalue) (Variables|Default|GetShieldPos) "None" "SnapToTarget" "SnapToTarget" "SnapToTarget" false)
  (Variables|/Game/RobotBattleContent/Assets/VFX/PlayerState/Shielding/BP_Shield.BP_Shield_C|SetRobot _returnvalue self)
  (Rendering|Components|Sprite|SetSprite (Variables|Default|GetTeamSprite) (Utilities|Select :Index (Variables|Default|GetTeam) :Option%200 "/Game/RobotBattleContent/Assets/Team/T_1_Sprite.T_1_Sprite" :Option%201 "/Game/RobotBattleContent/Assets/Team/T_2_Sprite1.T_2_Sprite1"))
  (Rendering|Material|SetMaterial (Variables|Character|GetMesh) 0 (Utilities|Select :Index (Variables|Default|GetTeam) :Option%200 "/Game/RobotBattleContent/Assets/Textures/RobotTexture/Top_S/Team1/M_TopS_T1.M_TopS_T1" :Option%201 "/Game/RobotBattleContent/Assets/Textures/RobotTexture/Top_S/Team2/M_TopS_T2.M_TopS_T2")))

(fn ConstructionScript)